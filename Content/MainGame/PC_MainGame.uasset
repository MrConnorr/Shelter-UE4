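; Player controller for a shelter survival game that rolls each player's character and feeds the main game widget.
; On local BeginPlay it loads the saved username and shows the widget; trait pools are filled from ShelterContent data-table columns.
; SetupPlayer combines uniform and weighted map picks, adjusting Russian wording and health by gender and age.
; Other events forward setup requests to GM_MainGame or push shelter, apocalypse and ace-card data into the UI.
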(event `SetUsername`
  ;[1 1 1] Sets Username
  (set `/Game/Blueprints/WBP_MainGame.Username` (`|FormatText` "{Username}#{PlayerID}" (`.Username_4_D60BC3C54AE1DACE04FB81A9F5EBAB98` (break `/Game/Player/PlayerInfo` (`self.PlayerSettings`))) (`AdvancedSessionsLibrary.GetPlayerName` (`GameplayStatics.GetPlayerController` 0))) (`self.MainGameRef`)))

(event `self.ReceiveBeginPlay`
  (bind _asshelter_game_instance (cast `/Game/Player/ShelterGameInstance` (`GameplayStatics.GetGameInstance`) :!pure true))
  (bind _loadingscreenref (`/Game/Player/ShelterGameInstance.LoadingScreenRef` (cast `/Game/Player/ShelterGameInstance` (`GameplayStatics.GetGameInstance`) :!pure true)))
  (`|ExecutionSequence`
    (:`then_0`
      ;[1 1 1] Loads player info and passes to serverside
      (`KismetSystemLibrary.Delay` 0.5)
      (if (`self.IsLocalController`)
        (`self.LoadGame`)
        (`/Game/Player/ShelterGameInstance.ShowMainGameWidget` _asshelter_game_instance)
        (set `self.MainGameRef` (`/Game/Player/ShelterGameInstance.MainGameRef` _asshelter_game_instance))
        (`self.SetUsername`)
        (`KismetSystemLibrary.Delay` 1.0)
        (`/Engine/EditorBlueprintResources/StandardMacros.IsValid` _loadingscreenref
          (:`Is Valid`
            (`Widget.RemoveFromParent` _loadingscreenref)))))
    (:`then_1`
      (bind _returnvalue (`DataTableFunctionLibrary.GetDataTableColumnAsString` "/Game/Data/ShelterContent.ShelterContent" "Occupation"))
      (`self.FillArray` _returnvalue (`self.OccupationArray`)))
    (:`then_2`
      (bind _returnvalue_2 (`DataTableFunctionLibrary.GetDataTableColumnAsString` "/Game/Data/ShelterContent.ShelterContent" "Health"))
      (`self.FillArray` _returnvalue_2 (`self.HealthArray`)))
    (:`then_3`
      (bind _returnvalue_3 (`DataTableFunctionLibrary.GetDataTableColumnAsString` "/Game/Data/ShelterContent.ShelterContent" "Hobby"))
      (`self.FillArray` _returnvalue_3 (`self.HobbyArray`)))
    (:`then_4`
      (bind _returnvalue_4 (`DataTableFunctionLibrary.GetDataTableColumnAsString` "/Game/Data/ShelterContent.ShelterContent" "Traits"))
      (`self.FillArray` _returnvalue_4 (`self.TraitsArray`)))
    (:`then_5`
      (bind _returnvalue_5 (`DataTableFunctionLibrary.GetDataTableColumnAsString` "/Game/Data/ShelterContent.ShelterContent" "Phobia"))
      (`self.FillArray` _returnvalue_5 (`self.PhobiaArray`)))
    (:`then_6`
      (bind _returnvalue_6 (`DataTableFunctionLibrary.GetDataTableColumnAsString` "/Game/Data/ShelterContent.ShelterContent" "AdditionalInfo"))
      (`self.FillArray` _returnvalue_6 (`self.AdditionalInfoArray`)))
    (:`then_7`
      (bind _returnvalue_7 (`DataTableFunctionLibrary.GetDataTableColumnAsString` "/Game/Data/ShelterContent.ShelterContent" "Backpack"))
      (`self.FillArray` _returnvalue_7 (`self.BackpackArray`)))))

(event `SetupApoc`
  (params (ApocDescritpion :type String))
  (set `/Game/Blueprints/WBP_MainGame.ApocalypseDescription` ApocDescritpion (`self.MainGameRef`)))

(event `SetupGame`
  (`/Game/MainGame/GM_MainGame.SetupGame` (cast `/Game/MainGame/GM_MainGame` (`GameplayStatics.GetGameMode`) :!pure true)))

(event `SetupSpecificPlayer`
  (params (PlayerID :type String) (IsNewPlayer :type Boolean))
  (`/Game/MainGame/GM_MainGame.SetupSpecificPlayer` (cast `/Game/MainGame/GM_MainGame` (`GameplayStatics.GetGameMode`) :!pure true) PlayerID IsNewPlayer))

(event `SetupShelter`
  (params (ShelterName :type String) (ShelterSize :type Integer) (ShelterPeople :type Integer) (ShelterCalendar :type String) (ShelterLocation :type String) (ShelterResources :type String) (ShelterMedicalStatus :type String) (ShelterFoodStatus :type String) (ShelterBedsStatus :type String) (ShelterWeaponStatus :type String) (ShelterChemicalStatus :type String))
  (bind _maingameref (`self.MainGameRef`))
  (set `/Game/Blueprints/WBP_MainGame.ShelterName` ShelterName _maingameref)
  (set `/Game/Blueprints/WBP_MainGame.ShelterSize` (`KismetTextLibrary.Conv_TextToString` (`|FormatText` "{ShelterSize} м²" ShelterSize)) _maingameref)
  (set `/Game/Blueprints/WBP_MainGame.ShelterPeople` (`KismetTextLibrary.Conv_TextToString` (`|FormatText` "{ShelterPeople} чел." ShelterPeople)) _maingameref)
  (set `/Game/Blueprints/WBP_MainGame.ShelterCalendar` ShelterCalendar _maingameref)
  (set `/Game/Blueprints/WBP_MainGame.ShelterLocation` (`KismetTextLibrary.Conv_TextToString` (`|FormatText` "Местонахождение бункера: \n{ShelterLocation}" ShelterLocation)) _maingameref)
  (set `/Game/Blueprints/WBP_MainGame.ShelterResources` (`KismetTextLibrary.Conv_TextToString` (`|FormatText` "Доступные ресурсы: \n{ShelterResources}" ShelterResources)) _maingameref)
  (set `/Game/Blueprints/WBP_MainGame.ShelterDescription` (`KismetTextLibrary.Conv_TextToString` (`|FormatText` "Помещения: \n{ShelterMedicalStatus}, \n{ShelterFoodStatus}, \n{ShelterBedsStatus}, \n{ShelterWeaponStatus}, \n{ShelterChemicalStatus}, \nЗапасов хватит на {ShelterPeople} человек на {ShelterCalendar}" ShelterMedicalStatus ShelterFoodStatus ShelterBedsStatus ShelterWeaponStatus ShelterChemicalStatus ShelterPeople ShelterCalendar)) _maingameref))

(event `SetAceCardsFromServer`
  (params (AceCard1 :type String) (AceCard2 :type String))
  (bind _maingameref (`self.MainGameRef`))
  (set `/Game/Blueprints/WBP_MainGame.AceCard1` AceCard1 _maingameref)
  (set `/Game/Blueprints/WBP_MainGame.AceCard2` AceCard2 _maingameref))

(event `UpdateShelterPeople`
  (params (ShelterPeople :type Integer))
  (set `/Game/Blueprints/WBP_MainGame.ShelterPeople` (`KismetTextLibrary.Conv_TextToString` (`|FormatText` "{ShelterPeople} чел." ShelterPeople)) (`self.MainGameRef`)))

(event `HideDIsableNotification`
  (bind _maingameref (`self.MainGameRef`))
  (`UserWidget.PlayAnimation` _maingameref (`/Game/Blueprints/WBP_MainGame.ShowNotification` _maingameref) 1.0 1 "Reverse" 1.0 false))

(event `SetupPlayer`
  (bind _maingameref (`self.MainGameRef`))
  (bind _outage (`self.FormatAge`))
  (bind _valueout (`self.RandomFromMap` (`self.GenderTable`)))
  (bind _genderout (`self.FormatGender` _valueout))
  (bind _valueout_2 (`self.RandomFromMap` (`self.SexualOrientationTable`)))
  (bind _sexualorientationout (`self.Format Sexual Orientation` _valueout_2 _genderout))
  (bind _occupationout (`self.FormatOccupation` (`KismetArrayLibrary.Array_Random` (`self.OccupationArray`)) _genderout))
  (bind _valueout_3 (`self.RandomFromMap` (`self.OccupationExperienceTable`)))
  (set `/Game/Blueprints/WBP_MainGame.Occupation` (`KismetTextLibrary.Conv_TextToString` (`|FormatText` "{Occupation} ({Experience})" _occupationout _valueout_3)) _maingameref)
  (set `/Game/Blueprints/WBP_MainGame.BiologicalCharacteristics` (`KismetTextLibrary.Conv_TextToString` (`|FormatText` "{Gender}/ {Age}/ \n{SexualOrientation}" _genderout _outage _sexualorientationout)) _maingameref)
  (bind _healthout (`self.Format Health` _genderout (`KismetArrayLibrary.Array_Random` (`self.HealthArray`)) _outage))
  (set `/Game/Blueprints/WBP_MainGame.Health` _healthout _maingameref)
  (set `/Game/Blueprints/WBP_MainGame.Hobby` (`KismetArrayLibrary.Array_Random` (`self.HobbyArray`)) _maingameref)
  (set `/Game/Blueprints/WBP_MainGame.Traits` (`KismetArrayLibrary.Array_Random` (`self.TraitsArray`)) _maingameref)
  (set `/Game/Blueprints/WBP_MainGame.Phobia` (`KismetArrayLibrary.Array_Random` (`self.PhobiaArray`)) _maingameref)
  (set `/Game/Blueprints/WBP_MainGame.AdditionalInfo` (`KismetArrayLibrary.Array_Random` (`self.AdditionalInfoArray`)) _maingameref)
  (set `/Game/Blueprints/WBP_MainGame.Backpack` (`KismetArrayLibrary.Array_Random` (`self.BackpackArray`)) _maingameref))

(event `EnableStatsButtons`
  (`Widget.SetIsEnabled` (`/Game/Blueprints/WBP_MainGame.BackpackBtn` (`self.MainGameRef`)) true)
  (`Widget.SetIsEnabled` (`/Game/Blueprints/WBP_MainGame.AdditionalInfoBtn` (`self.MainGameRef`)) true)
  (`Widget.SetIsEnabled` (`/Game/Blueprints/WBP_MainGame.BiologicalCharacteristicsBtn` (`self.MainGameRef`)) true)
  (`Widget.SetIsEnabled` (`/Game/Blueprints/WBP_MainGame.HealthBtn` (`self.MainGameRef`)) true)
  (`Widget.SetIsEnabled` (`/Game/Blueprints/WBP_MainGame.PhobiaBtn` (`self.MainGameRef`)) true)
  (`Widget.SetIsEnabled` (`/Game/Blueprints/WBP_MainGame.HobbyBtn` (`self.MainGameRef`)) true)
  (`Widget.SetIsEnabled` (`/Game/Blueprints/WBP_MainGame.TraitsBtn` (`self.MainGameRef`)) true)
  (`Widget.SetIsEnabled` (`/Game/Blueprints/WBP_MainGame.AceCard1Btn` (`self.MainGameRef`)) true)
  (`Widget.SetIsEnabled` (`/Game/Blueprints/WBP_MainGame.AceCard2Btn` (`self.MainGameRef`)) true)
  (`Widget.SetIsEnabled` (`/Game/Blueprints/WBP_MainGame.OccupationButton` (`self.MainGameRef`)) true))

(fn `CalculateSum`
  (params (MapIn :type "Map of String to Float (double-precision)"))
  (returns (Sum :type "Float (double-precision)"))
  (locals (RunningTotal :type "Float (double-precision)"))
  (bind _values (`BlueprintMapLibrary.Map_Values` MapIn))
  (for _array_element _values
    (set `local.RunningTotal` (+ (`local.RunningTotal`) _array_element)))
  (return (`local.RunningTotal`)))

(fn `ChooseFromMap`
  (params (ValueSum :type "Float (double-precision)") (MapIn :type "Map of String to Float (double-precision)"))
  (returns (ValueOut :type String))
  (locals (RandomValue :type "Float (double-precision)" :default 0.0) (MapElement :type String))
  (bind _value (`BlueprintMapLibrary.Map_Find` MapIn (`local.MapElement`)))
  (set `local.RandomValue` (`KismetMathLibrary.RandomFloatInRange` 0.0 ValueSum))
  (bind _keys (`BlueprintMapLibrary.Map_Keys` MapIn))
  (for _array_element _keys
    (set `local.MapElement` _array_element)
    (if (<= (`local.RandomValue`) _value)
      (return (`local.MapElement`))
      (else
        (set `local.RandomValue` (- (`local.RandomValue`) _value))))))

(fn `FillArray`
  (params (DataTableArray :type "Array of String") (ArrayToFill :type "Array of String"))
  (for _array_element DataTableArray
    (`KismetArrayLibrary.Array_Add` ArrayToFill _array_element)
    (if (`KismetStringLibrary.EqualEqual_StrStr` _array_element)
      (`KismetArrayLibrary.Array_RemoveItem` ArrayToFill _array_element)))
  (return))

(fn `Format Health`
  (params (GenderIn :type String) (HealthIn :type String) (AgeIn :type String))
  (returns (HealthOut :type String))
  (locals (Health :type String))
  (switch `string` GenderIn
    (:`Default`
      (set `local.Health` HealthIn))
    (:`Женщина`
      (if (and (`KismetStringLibrary.NotEqual_StrStr` HealthIn "Бесплодный") (>= (`KismetStringLibrary.Conv_StringToInt` AgeIn) 50))
        (set `local.Health` (`KismetTextLibrary.Conv_TextToString` (`|FormatText` "{Health}, Бесплодная" HealthIn)))
        (elif (and (`KismetStringLibrary.NotEqual_StrStr` HealthIn "Бесплодный") (<= (`KismetMathLibrary.RandomIntegerInRange` 0 100) 15))
          (set `local.Health` (`KismetTextLibrary.Conv_TextToString` (`|FormatText` "{Health}, Беременная" HealthIn)))
          (else
            (set `local.Health` HealthIn))))))
  (return (`local.Health`)))

(fn `Format Sexual Orientation`
  (params (SexualOrientationIn :type String) (GenderIn :type String))
  (returns (SexualOrientationOut :type String))
  (switch `string` SexualOrientationIn
    (:`Default`
      (set `self.Sexual Orientation Out` SexualOrientationIn))
    (:`гетеросексуальный(ная)`
      (switch `string` GenderIn
        (:`Default`
          (set `self.Sexual Orientation Out` "гетеросексуальный(ная)"))
        (:`Мужчина`
          (set `self.Sexual Orientation Out` "гетеросексуальный"))
        (:`Женщина`
          (set `self.Sexual Orientation Out` "гетеросексуальная"))))
    (:`гомосексуальный(ная)`
      (switch `string` GenderIn
        (:`Default`
          (set `self.Sexual Orientation Out` "гомосексуальный(ная)"))
        (:`Мужчина`
          (set `self.Sexual Orientation Out` "гомосексуальный"))
        (:`Женщина`
          (set `self.Sexual Orientation Out` "гомосексуальная")))))
  (return (`self.Sexual Orientation Out`)))

(fn `FormatAge`
  (returns (OutAge :type String))
  (locals (Age :type String) (RandomAge :type Integer :default 0))
  (bind _randomage (`local.RandomAge`))
  (set `local.RandomAge` (`KismetMathLibrary.RandomIntegerInRange` 20 70))
  (switch `int` (`KismetStringLibrary.Conv_StringToInt` (`KismetStringLibrary.Right` (`KismetStringLibrary.Conv_IntToString` (`local.RandomAge`)) 1))
    (:`0`
      (set `local.Age` (`KismetTextLibrary.Conv_TextToString` (`|FormatText` "{Age} лет" _randomage)) :!label _label))
    (:`1`
      (set `local.Age` (`KismetTextLibrary.Conv_TextToString` (`|FormatText` "{Age} год" _randomage))))
    (:`2`
      (set `local.Age` (`KismetTextLibrary.Conv_TextToString` (`|FormatText` "{Age} года" (`local.RandomAge`))) :!label _label_2))
    (:`3`
      (goto _label_2))
    (:`4`
      (goto _label_2))
    (:`5`
      (goto _label))
    (:`6`
      (goto _label))
    (:`7`
      (goto _label))
    (:`8`
      (goto _label))
    (:`9`
      (goto _label)))
  (return (`local.Age`)))

(fn `FormatGender`
  (params (GenderIn :type String))
  (returns (GenderOut :type String))
  (if (`KismetStringLibrary.EqualEqual_StrStr` GenderIn "Не определился")
    (set `self.Gender Out` (`KismetTextLibrary.Conv_TextToString` (`|FormatText` "Не определился ({FirstGender})" (`KismetArrayLibrary.Array_Random` (`|MakeArray` "Мужчина" "Женщина")))))
    (else
      (set `self.Gender Out` GenderIn)))
  (return (`self.Gender Out`)))

(fn `FormatOccupation`
  (params (OccupationIn :type String) (GenderIn :type String))
  (returns (OccupationOut :type String))
  (switch `string` OccupationIn
    (:`Default`
      (set `self.Occupation Out` OccupationIn))
    (:`Актёр/Актриса`
      (switch `string` GenderIn
        (:`Default`
          (set `self.Occupation Out` "Актёр/Актриса"))
        (:`Мужчина`
          (set `self.Occupation Out` "Актёр"))
        (:`Женщина`
          (set `self.Occupation Out` "Актриса"))))
    (:`Стриптизёр/Стриптизёрша`
      (switch `string` GenderIn
        (:`Default`
          (set `self.Occupation Out` "Стриптизёр/Стриптизёрша"))
        (:`Мужчина`
          (set `self.Occupation Out` "Стриптизёр"))
        (:`Женщина`
          (set `self.Occupation Out` "Стриптизёрша")))))
  (return (`self.Occupation Out`)))

(fn `LoadGame`
  (bind _returnvalue (`GameplayStatics.LoadGameFromSlot` "ShelterSettings"))
  (bind _asplayer_save (cast `/Game/Player/PlayerSave` _returnvalue))
  (set `self.PlayerSettings` (`/Game/Player/PlayerSave.S_PlayerInfo` _asplayer_save)))

(fn `RandomFromMap`
  (params (MapIn :type "Map of String to Float (double-precision)"))
  (returns (ValueOut :type String))
  (bind _sum (`self.CalculateSum` MapIn))
  (bind _valueout (`self.ChooseFromMap` _sum MapIn))
  (return _valueout))

(fn `UserConstructionScript`)