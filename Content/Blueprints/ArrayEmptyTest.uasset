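; A debug test Blueprint that reads the AceCards column from the ShelterContent data table and deals it into two card arrays.
; K collects the non-empty strings, printing each and calling SetupAceCards, which rebuilds both arrays by even and odd index, on every loop pass.
; L and M print each array, while O prints the first with a delay between entries.
; A Shuffle node is left unconnected.
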(event `Key|K`
  (params (Key :type "Key Structure"))
  (:`Pressed`
    (bind _returnvalue (`DataTableFunctionLibrary.GetDataTableColumnAsString` "/Game/Data/ShelterContent.ShelterContent" "AceCards"))
    (for _array_element _returnvalue
      (`KismetArrayLibrary.Array_Add` (`self.NewVar_0`) _array_element)
      (if (`KismetStringLibrary.EqualEqual_StrStr` _array_element)
        (`KismetArrayLibrary.Array_RemoveItem` (`self.NewVar_0`) _array_element)))
    (for (_array_element_2 _array_index) (`self.NewVar_0`)
      (`KismetSystemLibrary.PrintString` (`KismetStringLibrary.Concat_StrStr` (`KismetStringLibrary.Conv_IntToString` _array_index) " " _array_element_2))
      (`self.SetupAceCards`))))

(event `Key|L`
  (params (Key :type "Key Structure"))
  (:`Pressed`
    (for (_array_element _array_index) (`self.AceCards1Array`)
      (`KismetSystemLibrary.PrintString` (`KismetStringLibrary.Concat_StrStr` (`KismetStringLibrary.Conv_IntToString` _array_index) " " _array_element)))))

(event `Key|M`
  (params (Key :type "Key Structure"))
  (:`Pressed`
    (for (_array_element _array_index) (`self.AceCards2Array`)
      (`KismetSystemLibrary.PrintString` (`KismetStringLibrary.Concat_StrStr` (`KismetStringLibrary.Conv_IntToString` _array_index) " " _array_element)))))

(event `Key|O`
  (params (Key :type "Key Structure"))
  (:`Pressed`
    (bind (_array_element _array_index) (`/Game/Blueprints/BPM_ForEachWithLoop.ForEachLoopWithDelay` (`self.AceCards1Array`) 4.0)
      (:`Loop Body`
        (`KismetSystemLibrary.PrintString` (`KismetStringLibrary.Concat_StrStr` (`KismetStringLibrary.Conv_IntToString` _array_index) " " _array_element))))))

(event `SetupAceCards`
  (`KismetArrayLibrary.Array_Clear` (`self.AceCards1Array`))
  (`KismetArrayLibrary.Array_Clear` (`self.AceCards2Array`))
  (for (_array_element _array_index) (`self.NewVar_0`)
    (if (== (mod _array_index 2) 0)
      (`KismetArrayLibrary.Array_Add` (`self.AceCards1Array`) _array_element)
      (else
        (`KismetArrayLibrary.Array_Add` (`self.AceCards2Array`) _array_element)))))

(fn `UserConstructionScript`)