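; Lobby game mode that tracks joining and leaving players, shares match settings, and launches the main game once everyone is ready.
; It stores PC_Lobby controllers and pushes settings and player counts to each.
; EveryoneUpdated rebuilds the player list, optionally plays a random connect sound, and starts a short countdown, cancelled by any status other than "Готов" (Ready).
; When the timer fires, clients show a loading screen and servertravel opens L_MainGame.
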(event `self.K2_OnLogout`
  (params (ExitingController :type "Controller Object Reference"))
  (bind _aspc_lobby (cast `/Game/Lobby/PC_Lobby` ExitingController))
  (`KismetArrayLibrary.Array_RemoveItem` (`self.AllPlayerControllers`) _aspc_lobby)
  (`self.EveryoneUpdated` false))

(event `ServerUpdateGameSettings`
  (params (NumOfPlayers :type Integer) (AnswerTime :type "Float (double-precision)") (DecisionTime :type "Float (double-precision)"))
  (set `self.GMMaxNumOfPlayers` NumOfPlayers)
  (set `self.GMAnswerTime` AnswerTime)
  (set `self.GMDecisionTime` DecisionTime)
  (for _array_element (`self.AllPlayerControllers`)
    (bind _aspc_lobby (cast `/Game/Lobby/PC_Lobby` _array_element))
    (`/Game/Lobby/PC_Lobby.UpdateLobbySettings` _aspc_lobby (`self.GMMaxNumOfPlayers`) (`self.GMAnswerTime`) (`self.GMDecisionTime`))
    (`/Game/Lobby/PC_Lobby.UpdateNumOfPlayers` _aspc_lobby (`self.CurrentPlayers`) (`self.GMMaxNumOfPlayers`))))

(event `self.K2_PostLogin`
  (params (NewPlayer :type "PlayerController Object Reference"))
  ;[1 1 1] Initial setup
  (`/Engine/EditorBlueprintResources/ActorMacros.Switch Has Authority`
    (:`Authority`
      (`KismetArrayLibrary.Array_Add` (`self.AllPlayerControllers`) NewPlayer)
      (bind _aspc_lobby (cast `/Game/Lobby/PC_Lobby` NewPlayer))
      (`/Game/Lobby/PC_Lobby.InitialSetup` _aspc_lobby)
      (`/Game/Lobby/PC_Lobby.SetupLobby` _aspc_lobby)
      (`/Game/Lobby/PC_Lobby.UpdateLobbySettings` _aspc_lobby (`self.GMMaxNumOfPlayers`) (`self.GMAnswerTime`) (`self.GMDecisionTime`)))))

(event `LaunchGameMap`
  ;[1 1 1] Launch Game Map
  (`KismetSystemLibrary.ExecuteConsoleCommand` "servertravel /Game/Maps/L_MainGame" (`GameplayStatics.GetPlayerController` 0)))

(event `EveryoneUpdated`
  (params (PlayConnectSound :type Boolean))
  (bind _allplayercontrollers (`self.AllPlayerControllers`))
  (bind _output_get (set `self.CurrentPlayers` (`KismetArrayLibrary.Array_Length` (`self.AllPlayerControllers`))))
  (if (> _output_get 0)
    (`KismetArrayLibrary.Array_Clear` (`self.ConnectedPlayers`))
    (for _array_element _allplayercontrollers
      (bind _aspc_lobby (cast `/Game/Lobby/PC_Lobby` _array_element))
      (`KismetArrayLibrary.Array_Add` (`self.ConnectedPlayers`) (`/Game/Lobby/PC_Lobby.PlayerSettings` _aspc_lobby))
      (`/Game/Lobby/PC_Lobby.UpdateNumOfPlayers` _aspc_lobby (`self.CurrentPlayers`) (`self.GMMaxNumOfPlayers`)))
    (for _array_element_2 _allplayercontrollers
      (bind _aspc_lobby_2 (cast `/Game/Lobby/PC_Lobby` _array_element_2))
      (`/Game/Lobby/PC_Lobby.AddPlayerInfo` _aspc_lobby_2 (`self.ConnectedPlayers`))
      (if PlayConnectSound
        (bind _output_get_2 (set `self.RandomSound` (`KismetArrayLibrary.Array_Random` (`self.PlayerConnect`))))
        (`/Game/Lobby/PC_Lobby.PlaySoundOnPlayerConnect` _aspc_lobby_2 _output_get_2)))
    (for _array_element_3 (`self.ConnectedPlayers`) :!label _label
      (if (`KismetStringLibrary.EqualEqual_StrStr` (`.Status_5_5BA5BE6B4233F838215C41B6A2151D37` (break `/Game/Player/PlayerInfo` _array_element_3)) "Готов")
        (bind _returnvalue (`KismetSystemLibrary.K2_SetTimerDelegate` (delegate `StartGame`) 3.0))
        (bind _output_get_3 (set `self.StartGameTImer` _returnvalue))
        (for _array_element_4 (`self.AllPlayerControllers`)
          (bind _aspc_lobby_3 (cast `/Game/Lobby/PC_Lobby` _array_element_4))
          (`/Game/Lobby/PC_Lobby.ShowTimerOnClient` _aspc_lobby_3 (+ (`KismetMathLibrary.FTrunc` (`KismetSystemLibrary.K2_GetTimerRemainingTimeHandle` _output_get_3)) 1) true))
        (else
          (`KismetSystemLibrary.K2_ClearAndInvalidateTimerHandle` (`self.StartGameTImer`))
          (`/Engine/EditorBlueprintResources/StandardMacros.IsValid` _aspc_lobby_3
            (:`Is Valid`
              (for _array_element_5 (`self.AllPlayerControllers`)
                (bind _aspc_lobby_4 (cast `/Game/Lobby/PC_Lobby` _array_element_5))
                (`/Game/Lobby/PC_Lobby.ShowTimerOnClient` _aspc_lobby_4 0 false)
                (`self.CannotStartGame` :!label _label_2)))
            (:`Is Not Valid`
              (goto _label_2))))))))

(event `CannotStartGame`
  (goto _label :!via `Break`))

(event `StartGame`
  (for _array_element (`self.AllPlayerControllers`)
    (bind _aspc_lobby (cast `/Game/Lobby/PC_Lobby` _array_element))
    (`/Game/Lobby/PC_Lobby.ShowLoadingScreen` _aspc_lobby))
  (`self.LaunchGameMap`))

(fn `UserConstructionScript`)